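; BP_Enemy is an AI pawn that wanders until it sees a pawn, then chases it and ends the game on reaching it.
; Patrol repeatedly moves to random reachable points nearby, retrying on failure and pausing after success.
; PawnSensing sight triggers a chase via AIMoveTo, whose success shows the WBP_GameOver widget with a mouse cursor.
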(event OnSeePawn(PawnSensing)
  (params (Pawn :type Pawn%20Object%20Reference))
  (CallFunction|TargetChase Pawn))

(event Custom|Start%20Patrol
  (bind _self self)
  (AI|AIMoveTo _self (.RandomLocation (AI|Navigation|GetRandomReachablePointinRadius (Transformation|GetActorLocation) 1.5e+03 0 0)) 0 5.0 false
    (:OnSuccess
      (Utilities|FlowControl|Delay 1.0))
    (:OnFail
      _))
  (CallFunction|StartPatrol _self))

(event Custom|Target%20Chase
  (params (TargetActor :type Actor%20Object%20Reference))
  (bind _returnvalue (Game|GetPlayerController 0))
  (AI|AIMoveTo self "0, 0, 0" TargetActor 1.2e+02 false
    (:OnSuccess
      (bind _returnvalue_2 (UserInterface|CreateWidget "/Game/Blueprints/AI/WBP_GameOver.WBP_GameOver_C"))
      (Input|SetInputModeGameandUI _returnvalue 0 "DoNotLock" false false)
      (Variables|/Script/Engine.PlayerController|SetbShowMouseCursor _returnvalue true)
      (UserInterface|Viewport|AddtoViewport _returnvalue_2 0))))

(event EventBeginPlay
  (CallFunction|StartPatrol))

(fn ConstructionScript)