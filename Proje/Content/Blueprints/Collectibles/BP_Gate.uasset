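; BP_Gate is a collectible-gated door that swings open once enough items have been collected.
; Each CollectItem call increments a counter, and reaching the maximum fires OpenDoor through a DoOnce so it triggers only once.
; OpenDoor plays a timeline that lerps the door's relative yaw to swing it open.
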(event Custom|Open%20Door
  (bind _door_rot (Timeline|OpenDoor Play)
    (:Update
      (Transformation|SetRelativeRotation (Variables|Default|GetDoor) (Math|Rotator|MakeRotator 0.0 0.0 (Math|Float|Lerp 0.0 1.3e+02 _door_rot)) false false))))

(event Custom|Collect%20Item
  (Math|Integer|IncrementInt (Variables|Default|GetCurrentItemsCol)
    (:%20%20
      (if (>= (Variables|Default|GetCurrentItemsCol) (Variables|Default|GetMaximumItemsCol_0))
        (Utilities|FlowControl|DoOnce false
          (:Completed
            (CallFunction|OpenDoor)))))))

(fn ConstructionScript)